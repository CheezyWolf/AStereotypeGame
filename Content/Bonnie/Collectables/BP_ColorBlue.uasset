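; BP_ColorBlue is the blue color collectable, hidden with collision off until the player character has HasStereo2.
; Tick polls that flag and uses a DoOnce to reveal the cube and enable its box trigger.
; Player overlap shows an interact widget and enables input on the actor.
; Pressing E opens the Color2 widget in UI-only cursor mode, sets HasBlue on the character and destroys the actor.
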(event `self.ReceiveBeginPlay`
  (bind _cube (`self.Cube`))
  (`|ExecutionSequence`
    (:`then_0`
      (bind _returnvalue (`|CreateWidget` "/Game/Bonnie/Widgets/Interact_WBP.Interact_WBP_C"))
      (set `self.InteractUI` _returnvalue))
    (:`then_1`
      ; Hide Cube
      (`SceneComponent.SetVisibility` _cube false false)
      (`PrimitiveComponent.SetCollisionEnabled` _cube "NoCollision")
      (`PrimitiveComponent.SetCollisionEnabled` (`self.BoxCollision`) "NoCollision"))))

(event `self.ReceiveTick`
  (params (DeltaSeconds :type "Float (single-precision)"))
  (bind _cube (`self.Cube`))
  ; Show Cube
  (bind _asbp_first_person_character (cast `/Game/FirstPerson/Blueprints/BP_FirstPersonCharacter` (`GameplayStatics.GetPlayerCharacter` 0)))
  (if (`/Game/FirstPerson/Blueprints/BP_FirstPersonCharacter.HasStereo2?` _asbp_first_person_character)
    (`/Engine/EditorBlueprintResources/StandardMacros.DoOnce` false
      (:`Completed`
        (`SceneComponent.SetVisibility` _cube true false)
        (`PrimitiveComponent.SetCollisionEnabled` _cube "QueryAndPhysics")
        (`PrimitiveComponent.SetCollisionEnabled` (`self.BoxCollision`) "QueryOnly")))))

(event `self.BoxCollision.OnComponentBeginOverlap`
  (params (OverlappedComponent :type "PrimitiveComponent Object Reference") (OtherActor :type "Actor Object Reference") (OtherComp :type "PrimitiveComponent Object Reference") (OtherBodyIndex :type Integer) (bFromSweep :type Boolean) (SweepResult :type "HitResult Structure (by ref)"))
  ; Show Interact Ui
  (if (== OtherActor (`GameplayStatics.GetPlayerCharacter` 0))
    (`UserWidget.AddToViewport` (`self.InteractUI`) 0)
    (`self.EnableInput` (`GameplayStatics.GetPlayerController` 0))))

(event `self.BoxCollision.OnComponentEndOverlap`
  (params (OverlappedComponent :type "PrimitiveComponent Object Reference") (OtherActor :type "Actor Object Reference") (OtherComp :type "PrimitiveComponent Object Reference") (OtherBodyIndex :type Integer))
  ; Show Interact Ui
  (if (== OtherActor (`GameplayStatics.GetPlayerCharacter` 0))
    (`Widget.RemoveFromParent` (`self.InteractUI`))
    (`self.DisableInput` (`GameplayStatics.GetPlayerController` 0) null)))

(event `Key|E`
  (params (Key :type "Key Structure"))
  (bind _returnvalue (`GameplayStatics.GetPlayerController` 0))
  ; Show Stereoptye
  (:`Pressed`
    (`|ExecutionSequence`
      (:`then_0`
        (bind _returnvalue_2 (`|CreateWidget` "/Game/Bonnie/Widgets/Color2_WBP.Color2_WBP_C"))
        (bind _output_get (set `self.Color2UI` _returnvalue_2))
        (`UserWidget.AddToViewport` _output_get 0)
        (`WidgetBlueprintLibrary.SetInputMode_UIOnlyEx` _returnvalue null)
        (set `PlayerController.bShowMouseCursor` true _returnvalue)
        (`PlayerController.SetMouseLocation` _returnvalue 500 500))
      (:`then_1`
        (bind _asbp_first_person_character (cast `/Game/FirstPerson/Blueprints/BP_FirstPersonCharacter` (`GameplayStatics.GetPlayerCharacter` 0)))
        (set `/Game/FirstPerson/Blueprints/BP_FirstPersonCharacter.HasBlue?` true _asbp_first_person_character)
        (`self.K2_DestroyActor`)))))

(fn `UserConstructionScript`)