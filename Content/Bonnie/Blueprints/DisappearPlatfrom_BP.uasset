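; Disappearing platform actor that drops out from under the player shortly after being stepped on.
; When the player enters the box trigger, the platform mesh switches to a light material, then after a short delay turns invisible and loses collision.
; Any end overlap on the box, with no player check, restores the default material and, after a longer delay, brings back visibility and collision.
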(event `self.ReceiveBeginPlay`)

(event `self.BoxCollision.OnComponentBeginOverlap`
  (params (OverlappedComponent :type "PrimitiveComponent Object Reference") (OtherActor :type "Actor Object Reference") (OtherComp :type "PrimitiveComponent Object Reference") (OtherBodyIndex :type Integer) (bFromSweep :type Boolean) (SweepResult :type "HitResult Structure (by ref)"))
  (bind _disappearplatform (`self.DisappearPlatform`))
  (if (== OtherActor (`GameplayStatics.GetPlayerCharacter` 0))
    (`PrimitiveComponent.SetMaterial` (`self.DisappearPlatform`) 0 "/Game/Bonnie/Blueprints/M_Light.M_Light")
    (`KismetSystemLibrary.Delay` 0.8)
    (`SceneComponent.SetVisibility` _disappearplatform false false)
    (`PrimitiveComponent.SetCollisionEnabled` _disappearplatform "NoCollision")))

(event `self.BoxCollision.OnComponentEndOverlap`
  (params (OverlappedComponent :type "PrimitiveComponent Object Reference") (OtherActor :type "Actor Object Reference") (OtherComp :type "PrimitiveComponent Object Reference") (OtherBodyIndex :type Integer))
  (bind _disappearplatform (`self.DisappearPlatform`))
  (`PrimitiveComponent.SetMaterial` (`self.DisappearPlatform`) 0 "/Game/FirstPerson/MI_FirstPersonColorway.MI_FirstPersonColorway")
  (`KismetSystemLibrary.Delay` 2.0)
  (`SceneComponent.SetVisibility` _disappearplatform true false)
  (`PrimitiveComponent.SetCollisionEnabled` _disappearplatform "QueryAndPhysics"))

(fn `UserConstructionScript`)