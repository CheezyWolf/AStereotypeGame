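; BP_Trigger is a trigger volume that shows a female dialogue widget when the player walks into it.
; It creates the FemaleDialogue_WBP widget on BeginPlay, adds it to the viewport when the player character overlaps BoxCollision and removes it when the overlap ends.
; Separate DoOnce gates on enter and exit, with no reset wired, limit the dialogue to a single show and hide.
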(event `self.ReceiveBeginPlay`
  (bind _returnvalue (`|CreateWidget` "/Game/Bonnie/Widgets/FemaleDialogue_WBP.FemaleDialogue_WBP_C"))
  (set `self.Dialogue` _returnvalue))

(event `self.BoxCollision.OnComponentBeginOverlap`
  (params (OverlappedComponent :type "PrimitiveComponent Object Reference") (OtherActor :type "Actor Object Reference") (OtherComp :type "PrimitiveComponent Object Reference") (OtherBodyIndex :type Integer) (bFromSweep :type Boolean) (SweepResult :type "HitResult Structure (by ref)"))
  (if (== OtherActor (`GameplayStatics.GetPlayerCharacter` 0))
    (`/Engine/EditorBlueprintResources/StandardMacros.DoOnce` false
      (:`Completed`
        (`UserWidget.AddToViewport` (`self.Dialogue`) 0)))))

(event `self.BoxCollision.OnComponentEndOverlap`
  (params (OverlappedComponent :type "PrimitiveComponent Object Reference") (OtherActor :type "Actor Object Reference") (OtherComp :type "PrimitiveComponent Object Reference") (OtherBodyIndex :type Integer))
  (if (== OtherActor (`GameplayStatics.GetPlayerCharacter` 0))
    (`/Engine/EditorBlueprintResources/StandardMacros.DoOnce` false
      (:`Completed`
        (`Widget.RemoveFromParent` (`self.Dialogue`))))))

(fn `UserConstructionScript`)