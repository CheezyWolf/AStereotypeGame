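; BP_Wall is a gate wall that moves down when the player walks into its trigger box with the HasStereo1 flag set.
; A timeline drives the actor's location between StartLocation and EndLocation, with no reverse on exit.
; Without the flag, overlap shows a WallInteract_WBP widget created at BeginPlay, and leaving the box removes it.
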(event `self.ReceiveBeginPlay`
  (bind _returnvalue (`|CreateWidget` "/Game/Bonnie/Widgets/WallInteract_WBP.WallInteract_WBP_C"))
  (set `self.WallInteractUI` _returnvalue))

(event `self.BoxCollision.OnComponentBeginOverlap`
  (params (OverlappedComponent :type "PrimitiveComponent Object Reference") (OtherActor :type "Actor Object Reference") (OtherComp :type "PrimitiveComponent Object Reference") (OtherBodyIndex :type Integer) (bFromSweep :type Boolean) (SweepResult :type "HitResult Structure (by ref)"))
  (if (== OtherActor (`GameplayStatics.GetPlayerCharacter` 0))
    (bind _asbp_first_person_character (cast `/Game/FirstPerson/Blueprints/BP_FirstPersonCharacter` OtherActor))
    (if (`/Game/FirstPerson/Blueprints/BP_FirstPersonCharacter.HasStereo1?` _asbp_first_person_character)
      ; Wall move down
      (bind (_direction _newtrack_2) (`Timeline|Timeline`)
        (:`Update`
          (`self.K2_SetActorLocation` (`KismetMathLibrary.VLerp` (`self.StartLocation`) (`self.EndLocation`) _newtrack_2))))
      (else
        (`UserWidget.AddToViewport` (`self.WallInteractUI`) 0)))))

(event `self.BoxCollision.OnComponentEndOverlap`
  (params (OverlappedComponent :type "PrimitiveComponent Object Reference") (OtherActor :type "Actor Object Reference") (OtherComp :type "PrimitiveComponent Object Reference") (OtherBodyIndex :type Integer))
  (if (== OtherActor (`GameplayStatics.GetPlayerCharacter` 0))
    (`Widget.RemoveFromParent` (`self.WallInteractUI`))))

(fn `UserConstructionScript`)