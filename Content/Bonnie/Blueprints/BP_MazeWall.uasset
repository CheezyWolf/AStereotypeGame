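; BP_MazeWall is a maze wall that slides upward once the player's first-person character has the second stereo (HasStereo2).
; Tick polls that flag on the player and, through a DoOnce, starts the Movement timeline a single time.
; Each timeline update lerps from the current location toward a point slightly above it, so the rise accumulates, and a second DoOnce plays a short sliding sound.
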(event `self.ReceiveTick`
  (params (DeltaSeconds :type "Float (single-precision)"))
  ; Maze Wall move up
  (bind _asbp_first_person_character (cast `/Game/FirstPerson/Blueprints/BP_FirstPersonCharacter` (`GameplayStatics.GetPlayerCharacter` 0)))
  (if (`/Game/FirstPerson/Blueprints/BP_FirstPersonCharacter.HasStereo2?` _asbp_first_person_character)
    (`/Engine/EditorBlueprintResources/StandardMacros.DoOnce` false
      (:`Completed`
        (bind (_direction _wallup) (`Timeline|Movement`)
          (:`Update`
            (`self.K2_SetActorLocation` (`KismetMathLibrary.VLerp` (`self.K2_GetActorLocation`) (+ (`self.K2_GetActorLocation`) (0.0 0.0 10.0)) _wallup))
            (`/Engine/EditorBlueprintResources/StandardMacros.DoOnce` false
              (:`Completed`
                (`GameplayStatics.PlaySound2D` "/Game/Bonnie/Audio/WallSlidingShort.WallSlidingShort" 1.0 1.0 0.0 null null)))))))))

(fn `UserConstructionScript`)