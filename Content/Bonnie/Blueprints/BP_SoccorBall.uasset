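; BP_SoccorBall is a soccer ball actor that the player can kick while standing near it.
; Overlapping BoxCollision with the player character enables input and opens a Gate, and leaving disables input and closes it.
; While the Gate is open, a left mouse press applies a velocity-change impulse to BallMesh along the player controller's forward vector, scaled by PassSpeed, and prints a debug message.
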(event `Key|LeftMouseButton`
  (params (Key :type "Key Structure"))
  (:`Pressed`
    (`/Engine/EditorBlueprintResources/StandardMacros.Gate` true :!label _label
      (:`Exit`
        ; Kick Soccer Ball
        (`PrimitiveComponent.AddImpulse` (`self.BallMesh`) (* (`self.GetActorForwardVector` (`GameplayStatics.GetPlayerController` 0)) (`self.PassSpeed`)) "None" true)
        (`KismetSystemLibrary.PrintString` "hit")))))

(event `self.BoxCollision.OnComponentBeginOverlap`
  (params (OverlappedComponent :type "PrimitiveComponent Object Reference") (OtherActor :type "Actor Object Reference") (OtherComp :type "PrimitiveComponent Object Reference") (OtherBodyIndex :type Integer) (bFromSweep :type Boolean) (SweepResult :type "HitResult Structure (by ref)"))
  (if (== OtherActor (`GameplayStatics.GetPlayerCharacter` 0))
    (`self.EnableInput` (`GameplayStatics.GetPlayerController` 0))
    (goto _label :!via `Open`)))

(event `self.BoxCollision.OnComponentEndOverlap`
  (params (OverlappedComponent :type "PrimitiveComponent Object Reference") (OtherActor :type "Actor Object Reference") (OtherComp :type "PrimitiveComponent Object Reference") (OtherBodyIndex :type Integer))
  (if (== (`GameplayStatics.GetPlayerCharacter` 0) OtherActor)
    (`self.DisableInput` (`GameplayStatics.GetPlayerController` 0))
    (goto _label :!via `Close`)))

(fn `UserConstructionScript`)