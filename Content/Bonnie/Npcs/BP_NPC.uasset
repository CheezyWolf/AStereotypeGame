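; BP_NPC is an NPC that falls dead the first time a BP_SoccorBall overlaps its capsule.
; The hit plays a death animation, disables capsule collision, destroys the actor after a delay and adds one to the player character's Score.
; When Score reaches three, it briefly shows the Saved_WBP widget created at BeginPlay and, after a delay, makes BP_Collectable2 visible with query collision.
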(event `self.ReceiveBeginPlay`
  (bind _returnvalue (`|CreateWidget` "/Game/Bonnie/Widgets/Saved_WBP.Saved_WBP_C"))
  (set `self.SavedUI` _returnvalue))

(event `self.CapsuleComponent.OnComponentBeginOverlap`
  (params (OverlappedComponent :type "PrimitiveComponent Object Reference") (OtherActor :type "Actor Object Reference") (OtherComp :type "PrimitiveComponent Object Reference") (OtherBodyIndex :type Integer) (bFromSweep :type Boolean) (SweepResult :type "HitResult Structure (by ref)"))
  ; Play Dead Anim
  (cast `/Game/Bonnie/Blueprints/BP_SoccorBall` OtherActor)
  (`/Engine/EditorBlueprintResources/StandardMacros.DoOnce` false
    (:`Completed`
      (`|ExecutionSequence`
        (:`then_0`
          (`SkeletalMeshComponent.PlayAnimation` (`self.Mesh`) "/Game/Bonnie/Animation/FallingBackDeath_Anim.FallingBackDeath_Anim" false)
          (`KismetSystemLibrary.Delay` 0.5)
          (`PrimitiveComponent.SetCollisionEnabled` (`self.CapsuleComponent`) "NoCollision")
          (`KismetSystemLibrary.Delay` 4.0)
          (`self.K2_DestroyActor`))
        (:`then_1`
          ; How many NPCs Died
          (bind _asbp_first_person_character (cast `/Game/FirstPerson/Blueprints/BP_FirstPersonCharacter` (`GameplayStatics.GetPlayerCharacter` 0)))
          (bind _output_get (set `/Game/FirstPerson/Blueprints/BP_FirstPersonCharacter.Score` (+ (`/Game/FirstPerson/Blueprints/BP_FirstPersonCharacter.Score` _asbp_first_person_character) 1) _asbp_first_person_character))
          (if (== _output_get 3)
            (`|ExecutionSequence`
              (:`then_0`
                ; Collectible 2 visible
                (bind _returnvalue (`GameplayStatics.GetActorOfClass` "/Game/Bonnie/Collectables/BP_Collectable2.BP_Collectable2_C"))
                (`KismetSystemLibrary.Delay` 4.0)
                (bind _cube (`/Game/Bonnie/Collectables/BP_Collectable2.Cube` _returnvalue))
                (`SceneComponent.SetVisibility` _cube true false)
                (`PrimitiveComponent.SetCollisionEnabled` _cube "QueryOnly")
                (`PrimitiveComponent.SetCollisionEnabled` (`/Game/Bonnie/Collectables/BP_Collectable2.BoxCollision` _returnvalue) "QueryOnly"))
              (:`then_1`
                (`KismetSystemLibrary.Delay` 1.0)
                (`UserWidget.AddToViewport` (`self.SavedUI`) 0)
                (`KismetSystemLibrary.Delay` 3.0)
                (`Widget.RemoveFromParent` (`self.SavedUI`))))))))))

(fn `UserConstructionScript`)